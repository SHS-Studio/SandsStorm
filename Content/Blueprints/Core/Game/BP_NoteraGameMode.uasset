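; Game mode for Notera that manages front-end screens, input modes and a one-time level cinematic.
; BeginPlay disables player input, grabs the first level sequence actor, shows the splash screen and binds the cinematic event.
; StartCinematics fires that event once, playing the sequence and delaying for its end time before restoring the character's animation Blueprint and input.
; Helper functions show title, splash, update and loading widgets, clear them, or switch input mode.
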(event Custom|EnableCinematics_Event
  (bind _levelsequence (Variables|Default|GetLevelSequence))
  (bind _sequenceplayer (Variables|/Script/LevelSequence.LevelSequenceActor|GetSequencePlayer _levelsequence))
  (Sequencer|Player|Play _sequenceplayer :!class /Script/MovieScene.MovieSceneSequencePlayer)
  (bind _asbp_notera_player_char (Utilities|Casting|CastToBpNoteraPlayerChar (Game|GetPlayerCharacter 0)))
  (Input|DisableInput _asbp_notera_player_char 0)
  (Utilities|FlowControl|Delay (Class|TimeManagementBlueprintLibrary|ToSeconds(QualifiedFrameTime) (Class|MovieSceneSequencePlayer|GetEndTime _sequenceplayer)))
  (Components|SkeletalMesh|SetAnimInstanceClass (Variables|/Script/Engine.Character|GetMesh _asbp_notera_player_char) "/Game/Character/AbpNoteraPlayerChar.AbpNoteraPlayerChar_C")
  (Components|Animation|SetAnimationMode (Variables|/Script/Engine.Character|GetMesh _asbp_notera_player_char) "AnimationBlueprint" true)
  (Input|EnableInput _asbp_notera_player_char 0))

(event EventBeginPlay
  (Utilities|FlowControl|Sequence
    (:then_0
      (bind _asbp_notera_player_char (Utilities|Casting|CastToBpNoteraPlayerChar (Game|GetPlayerCharacter 0)))
      (Input|DisableInput _asbp_notera_player_char 0))
    (:then_1
      (CallFunction|SetInputMode 1 :!label _label)
      (bind _outactors (Actor|GetAllActorsOfClass "/Script/LevelSequence.LevelSequenceActor"))
      (Variables|Default|SetLevelSequence (Utilities|Array|Get(acopy) _outactors))
      (CallFunction|EnableSplashScreen))
    (:then_2
      (EventDispatchers|BindEventtoEnableCinematics (delegate Custom|EnableCinematics_Event))
      (goto _label))))

(event EventTick
  (params (DeltaSeconds :type Float%20%28single-precision%29)))

(fn ConstructionScript)

(fn EnableTitleMenu
  (bind _titlemenuscreen (Variables|Default|GetTitleMenuScreen))
  (UserInterface|CreateWidget (Utilities|GetClass _titlemenuscreen))
  (UserInterface|Viewport|AddtoViewport _titlemenuscreen 0)
  (Widget|SetKeyboardFocus _titlemenuscreen)
  (Variables|Default|SetIsTitleScreenEnabled true))

(fn ResetScreen
  (Widget|RemovefromParent (Variables|Default|GetTitleMenuScreen))
  (Widget|RemovefromParent (Variables|Default|GetSplashScreen))
  (Widget|RemovefromParent (Variables|Default|GetGameUpdateScreen))
  (Widget|RemovefromParent (Variables|Default|GetLoadingScreen))
  (Variables|Default|SetIsTitleScreenEnabled false))

(fn EnableSplashScreen
  (bind _splashscreen (Variables|Default|GetSplashScreen))
  (UserInterface|CreateWidget (Utilities|GetClass _splashscreen))
  (UserInterface|Viewport|AddtoViewport _splashscreen 0))

(fn EnableGameUpdate
  (bind _gameupdatescreen (Variables|Default|GetGameUpdateScreen))
  (UserInterface|CreateWidget (Utilities|GetClass _gameupdatescreen))
  (UserInterface|Viewport|AddtoViewport _gameupdatescreen 0))

(fn EnableLoadingScreen
  (bind _returnvalue (UserInterface|CreateWidget (Utilities|GetClass (Variables|Default|GetLoadingScreen))))
  (UserInterface|Viewport|AddtoViewport _returnvalue 0))

(fn StartCinematics
  (if (Variables|Default|GetCanCineMaticsPlay)
    (Default|CallEnableCinematics)
    (Variables|Default|SetCanCineMaticsPlay false)))

(fn SetInputMode
  (params (Type :type Integer))
  (bind _returnvalue (Game|GetPlayerController 0))
  (if (== Type 0)
    (Input|SetInputModeUIOnly _returnvalue (Variables|Default|GetTitleMenuScreen) "LockAlways" false)
    (elif (== Type 1)
      (Input|SetInputModeGameandUI _returnvalue 0 "LockAlways" true false)
      (else
        (Input|SetInputModeGameOnly _returnvalue false)))))